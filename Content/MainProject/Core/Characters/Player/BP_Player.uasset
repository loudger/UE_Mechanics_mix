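; Player character Blueprint that zooms the camera out while sprinting.
; BeginPlay caches the spring arm's initial length as the default.
; Sprint start plays a timeline that lerps the arm length toward the sprint length, and sprint stop reverses the same timeline to ease it back from its current point.
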(event EventOnSprintStart
  ;[1 1 1] CameraOutZoomWhenSprinting
  (bind _newtrack_0 (Timeline|Spring%20arm%20sprint%20timeline Play)
    (:Update
      (Variables|/Script/Engine.SpringArmComponent|SetTargetArmLength (Variables|Default|GetSpringArmComponent) (Math|Float|Lerp (Variables|SprintSetting|GetDefaultArmLength) (Variables|SprintSetting|GetSprintArmLength) _newtrack_0)))))

(event EventBeginPlay
  ;[1 1 1] CameraOutZoomWhenSprinting
  (Variables|SprintSetting|SetDefaultArmLength (Variables|/Script/Engine.SpringArmComponent|GetTargetArmLength (Variables|Default|GetSpringArmComponent))))

(event EventOnSprintStop
  ;[1 1 1] CameraOutZoomWhenSprinting
  (bind _newtrack_0 (Timeline|Spring%20arm%20sprint%20timeline Reverse)
    (:Update
      (Variables|/Script/Engine.SpringArmComponent|SetTargetArmLength (Variables|Default|GetSpringArmComponent) (Math|Float|Lerp (Variables|SprintSetting|GetDefaultArmLength) (Variables|SprintSetting|GetSprintArmLength) _newtrack_0)))))

(fn ConstructionScript)